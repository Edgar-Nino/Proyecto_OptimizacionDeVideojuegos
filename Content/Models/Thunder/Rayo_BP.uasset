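; Lightning (Rayo) actor that calls RayoFunc on the player character class BP_GRFH1_CharacterP when that character overlaps its Box, then destroys itself.
; If its owner is a Levitator_BP, it clears that owner's Full flag before being destroyed.
; Instances without a Levitator_BP owner destroy themselves after a short delay from BeginPlay, while levitator-owned ones persist until touched.
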(event `self.Box.OnComponentBeginOverlap`
  (params (OverlappedComponent :type "PrimitiveComponent Object Reference") (OtherActor :type "Actor Object Reference") (OtherComp :type "PrimitiveComponent Object Reference") (OtherBodyIndex :type Integer) (bFromSweep :type Boolean) (SweepResult :type "HitResult Structure (by ref)"))
  (if (== (`GameplayStatics.GetObjectClass` OtherActor) "/Game/GR_Stylized_Female_01/Character/Blueprints/BP_GRFH1_CharacterP.BP_GRFH1_CharacterP_C")
    (bind _asbp_grfh1_character_p (cast `/Game/GR_Stylized_Female_01/Character/Blueprints/BP_GRFH1_CharacterP` OtherActor))
    (`/Game/GR_Stylized_Female_01/Character/Blueprints/BP_GRFH1_CharacterP.Rayo_Func` _asbp_grfh1_character_p)
    (bind _aslevitator_bp (cast `/Game/Models/Levitador/Levitator_BP` (`self.GetOwner`))
      (:`then`
        (set `/Game/Models/Levitador/Levitator_BP.Full` false _aslevitator_bp))
      (:`CastFailed`
        _))
    (`self.K2_DestroyActor`)))

(event `self.ReceiveBeginPlay`
  (cast `/Game/Models/Levitador/Levitator_BP` (`self.GetOwner`)
    (:`CastFailed`
      (`KismetSystemLibrary.Delay` 5.0)
      (`self.K2_DestroyActor`))))

(fn `UserConstructionScript`)