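; Key pickup actor that the player collects with the Interaction input while standing inside its trigger box.
; Box overlap with BP_GRFH1_CharacterP enables input on the actor for player controller 0, and leaving the box disables it.
; Pressing Interaction spawns the Get_Key particle effect and a spatialized grab sound, then destroys the actor, without recording the pickup anywhere.
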(event `self.ReceiveBeginPlay`)

(event `InputAction|Interaction`
  (params (Key :type "Key Structure"))
  (bind _returnvalue (`self.K2_GetActorLocation`))
  (:`Pressed`
    (`GameplayStatics.SpawnEmitterAtLocation` "/Game/Particles/Ammo/Get_Key.Get_Key" _returnvalue)
    (`GameplayStatics.SpawnSoundAtLocation` "/Game/Sounds/GrabKey.GrabKey" _returnvalue (struct) 8.0 1.0 0.0 "/Game/Sounds/ProjectileAttenuation.ProjectileAttenuation" null)
    (`self.K2_DestroyActor`)))

(event `self.Box.OnComponentBeginOverlap`
  (params (OverlappedComponent :type "PrimitiveComponent Object Reference") (OtherActor :type "Actor Object Reference") (OtherComp :type "PrimitiveComponent Object Reference") (OtherBodyIndex :type Integer) (bFromSweep :type Boolean) (SweepResult :type "HitResult Structure (by ref)"))
  (if (== (`GameplayStatics.GetObjectClass` OtherActor) "/Game/GR_Stylized_Female_01/Character/Blueprints/BP_GRFH1_CharacterP.BP_GRFH1_CharacterP_C")
    (`self.EnableInput` (`GameplayStatics.GetPlayerController` 0))))

(event `self.Box.OnComponentEndOverlap`
  (params (OverlappedComponent :type "PrimitiveComponent Object Reference") (OtherActor :type "Actor Object Reference") (OtherComp :type "PrimitiveComponent Object Reference") (OtherBodyIndex :type Integer))
  (if (== (`GameplayStatics.GetObjectClass` OtherActor) "/Game/GR_Stylized_Female_01/Character/Blueprints/BP_GRFH1_CharacterP.BP_GRFH1_CharacterP_C")
    (`self.DisableInput` (`GameplayStatics.GetPlayerController` 0))))

(fn `UserConstructionScript`)