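; Homing projectile (Perseguidoras) that seeks Enemy_BP actors and, on hitting one, spawns an emitter and destroys itself.
; Every Tick, FindHomingTarget scans all non-destroyed enemies and feeds the chosen one's Destructible component to the Projectile movement component, disabling homing when none qualifies.
; Selection minimizes the distance between each enemy's actor origin and its own Destructible component, so the projectile's position plays no part.
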(event `MoveToTarget`
  (bind (_destructible _bool_none) (`self.FindHomingTarget`))
  (if _bool_none
    (set `ProjectileMovementComponent.bIsHomingProjectile` false (`self.Projectile`))
    (else
      (set `ProjectileMovementComponent.HomingTargetComponent` (`/Game/Models/Enemy/Enemy_BP.Destructible` _destructible) (`self.Projectile`))
      (set `ProjectileMovementComponent.bIsHomingProjectile` true (`self.Projectile`)))))

(event `self.ReceiveTick`
  (params (DeltaSeconds :type "Float (single-precision)"))
  (`self.MoveToTarget`))

(event `self.ReceiveHit`
  (params (MyComp :type "PrimitiveComponent Object Reference") (Other :type "Actor Object Reference") (OtherComp :type "PrimitiveComponent Object Reference") (bSelfMoved :type Boolean) (HitLocation :type "Vector Structure") (HitNormal :type "Vector Structure") (NormalImpulse :type "Vector Structure") (Hit :type "HitResult Structure (by ref)"))
  (if (== (`GameplayStatics.GetObjectClass` Other) "/Game/Models/Enemy/Enemy_BP.Enemy_BP_C")
    (`GameplayStatics.SpawnEmitterAtLocation` "/Game/Particles/Destroyed/Destroyed.Destroyed" HitLocation)
    (`self.K2_DestroyActor`)))

(fn `FindHomingTarget`
  (returns (Destructible :type "/Game/Models/Enemy/Enemy_BP Object Reference") (Bool_None :type Boolean))
  (locals (`Closest distance` :type "Float (double-precision)" :default 100000.0) (HomingTarget :type "/Game/Models/Enemy/Enemy_BP Object Reference"))
  (set `local.Closest distance` 100000.0)
  (bind _outactors (`GameplayStatics.GetAllActorsOfClass` "/Game/Models/Enemy/Enemy_BP.Enemy_BP_C"))
  (for _array_element _outactors
    (bind _asenemy_bp (cast `/Game/Models/Enemy/Enemy_BP` _array_element))
    (if (not (`/Game/Models/Enemy/Enemy_BP.Destroyed` _asenemy_bp))
      (bind _returnvalue (`KismetMathLibrary.VSize` (- (`self.K2_GetActorLocation` _asenemy_bp) (`SceneComponent.K2_GetComponentLocation` (`/Game/Models/Enemy/Enemy_BP.Destructible` _asenemy_bp)))))
      (if (< _returnvalue (`local.Closest distance`))
        (set `local.Closest distance` _returnvalue)
        (set `local.HomingTarget` _asenemy_bp))))
  (return (`local.HomingTarget`) (== (`local.Closest distance`) 100000.0)))

(fn `UserConstructionScript`)