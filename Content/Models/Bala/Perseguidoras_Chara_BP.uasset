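; Homing projectile that chases the nearest BP_GRFH1_CharacterP other than its instigator, playing a sound on spawn.
; Every tick it scans all characters for the closest and points the projectile movement's homing at its Skin component, disabling homing when none is found.
; Hitting another character spawns effects, hides and disables collision, adds a point to the instigator, damages the victim, then destroys the projectile after a delay.
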(event `MoveToTarget`
  (bind (_character _bool_none) (`self.FindHomingTarget`))
  (if _bool_none
    (set `ProjectileMovementComponent.bIsHomingProjectile` false (`self.Projectile`))
    (else
      (set `ProjectileMovementComponent.HomingTargetComponent` (`/Game/GR_Stylized_Female_01/Character/Blueprints/BP_GRFH1_CharacterP.skin` _character) (`self.Projectile`))
      (set `ProjectileMovementComponent.bIsHomingProjectile` true (`self.Projectile`)))))

(event `self.ReceiveTick`
  (params (DeltaSeconds :type "Float (single-precision)"))
  (`self.MoveToTarget`))

(event `self.ReceiveBeginPlay`
  (`GameplayStatics.PlaySoundAtLocation` "/Game/Sounds/Perseguidora.Perseguidora" (`self.K2_GetActorLocation`) (struct) 1.25 1.0 0.0 null null null))

(event `self.ReceiveHit`
  (params (MyComp :type "PrimitiveComponent Object Reference") (Other :type "Actor Object Reference") (OtherComp :type "PrimitiveComponent Object Reference") (bSelfMoved :type Boolean) (HitLocation :type "Vector Structure") (HitNormal :type "Vector Structure") (NormalImpulse :type "Vector Structure") (Hit :type "HitResult Structure (by ref)"))
  (`self.HitProjectile` Other HitLocation))

(event `HitProjectile`
  (params (ActorObject :type "Actor Object Reference") (VectorLoc :type "Vector Structure"))
  (if (`self.Destroyed`)
    _
    (elif (and (!= (`self.GetInstigator`) ActorObject) (== (`GameplayStatics.GetObjectClass` ActorObject) "/Game/GR_Stylized_Female_01/Character/Blueprints/BP_GRFH1_CharacterP.BP_GRFH1_CharacterP_C"))
      (`self.HitProjectileParticles` VectorLoc)
      (set `self.Destroyed` true)
      (`PrimitiveComponent.SetCollisionEnabled` (`self.CollisionComponent`) "NoCollision")
      (bind _asbp_grfh1_character_p (cast `/Game/GR_Stylized_Female_01/Character/Blueprints/BP_GRFH1_CharacterP` (`self.GetInstigator`)))
      (`/Engine/EditorBlueprintResources/StandardMacros.DoOnce` false
        (:`Completed`
          (`/Game/GR_Stylized_Female_01/Character/Blueprints/BP_GRFH1_CharacterP.ScoreUpdate` _asbp_grfh1_character_p 1)
          (bind _asbp_grfh1_character_p_2 (cast `/Game/GR_Stylized_Female_01/Character/Blueprints/BP_GRFH1_CharacterP` ActorObject))
          (`/Game/GR_Stylized_Female_01/Character/Blueprints/BP_GRFH1_CharacterP.DamageExec` _asbp_grfh1_character_p_2)
          (`KismetSystemLibrary.Delay` 2.0)
          (`self.K2_DestroyActor`))))))

(event `HitProjectileParticles`
  (params (VectorLoc :type "Vector Structure"))
  (`GameplayStatics.SpawnEmitterAtLocation` "/Game/Particles/Destroyed/Destroyed.Destroyed" VectorLoc)
  (`GameplayStatics.PlaySoundAtLocation` "/Game/Sounds/Hit.Hit" VectorLoc (struct) 1.0 1.0 0.0 "/Game/Sounds/ProjectileAttenuation.ProjectileAttenuation" null null)
  (`SceneComponent.SetVisibility` (`self.CollisionComponent`) false true))

(fn `FindHomingTarget`
  (returns (Character :type "/Game/GR_Stylized_Female_01/Character/Blueprints/BP_GRFH1_CharacterP Object Reference") (Bool_None :type Boolean))
  (locals (`Closest distance` :type "Float (double-precision)" :default 100000.0) (HomingTarget :type "/Game/GR_Stylized_Female_01/Character/Blueprints/BP_GRFH1_CharacterP Object Reference"))
  (set `local.Closest distance` 100000.0)
  (bind _outactors (`GameplayStatics.GetAllActorsOfClass` "/Game/GR_Stylized_Female_01/Character/Blueprints/BP_GRFH1_CharacterP.BP_GRFH1_CharacterP_C"))
  (for _array_element _outactors
    (if (not (== _array_element (`self.GetInstigator`)))
      (bind _asbp_grfh1_character_p (cast `/Game/GR_Stylized_Female_01/Character/Blueprints/BP_GRFH1_CharacterP` _array_element))
      (bind _returnvalue (`KismetMathLibrary.Vector_Distance` (`self.K2_GetActorLocation` _asbp_grfh1_character_p) (`self.K2_GetActorLocation`)))
      (if (< _returnvalue (`local.Closest distance`))
        (set `local.Closest distance` _returnvalue)
        (set `local.HomingTarget` _asbp_grfh1_character_p))))
  (return (`local.HomingTarget`) (== (`local.Closest distance`) 100000.0)))

(fn `UserConstructionScript`)