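; Life_BP is a health pickup actor that heals the player character on touch.
; Its Box overlap checks that the other actor's class matches the player's, then clears the Full flag on its owning Levitator_BP.
; It then calls CuracionFunc on BP_GRFH1_CharacterP and destroys itself.
; Both casts must succeed, so a pickup without a Levitator_BP owner neither heals nor disappears.
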(event `self.ReceiveTick`
  (params (DeltaSeconds :type "Float (single-precision)")))

(event `self.Box.OnComponentBeginOverlap`
  (params (OverlappedComponent :type "PrimitiveComponent Object Reference") (OtherActor :type "Actor Object Reference") (OtherComp :type "PrimitiveComponent Object Reference") (OtherBodyIndex :type Integer) (bFromSweep :type Boolean) (SweepResult :type "HitResult Structure (by ref)"))
  (bind _returnvalue (`GameplayStatics.GetPlayerCharacter` 0))
  (if (== (`GameplayStatics.GetObjectClass` OtherActor) (`GameplayStatics.GetObjectClass` _returnvalue))
    (bind _aslevitator_bp (cast `/Game/Models/Levitador/Levitator_BP` (`self.GetOwner`)))
    (set `/Game/Models/Levitador/Levitator_BP.Full` false _aslevitator_bp)
    (bind _asbp_grfh1_character_p (cast `/Game/GR_Stylized_Female_01/Character/Blueprints/BP_GRFH1_CharacterP` _returnvalue))
    (`/Game/GR_Stylized_Female_01/Character/Blueprints/BP_GRFH1_CharacterP.Curacion_Func` _asbp_grfh1_character_p)
    (`self.K2_DestroyActor`)))

(fn `UserConstructionScript`)