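; Animated gyro plant Blueprint that spins a crystal and rocks two pivot components for decorative motion.
; Each Tick yaws GyroCrystal at VelocityRot and adds delta time to a running clock.
; That clock drives sine-based roll, pitch and yaw on Empty, with Empty1 receiving the negated rotation so the two swing in opposition.
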(event `self.ReceiveTick`
  (params (DeltaSeconds :type "Float (single-precision)"))
  (bind _returnvalue (`KismetMathLibrary.DegSin` (* (`self.Local`) 30.0)))
  (bind _returnvalue_2 (* 30.0 _returnvalue))
  (bind _returnvalue_3 (* _returnvalue_2 -1.0))
  (bind _returnvalue_4 (* (`KismetMathLibrary.DegAtan` _returnvalue) 5.0))
  (set `self.Local` (+ DeltaSeconds (`self.Local`)))
  (`SceneComponent.K2_AddLocalRotation` (`self.Gyro_Crystal`) (`KismetMathLibrary.MakeRotator` 0.0 0.0 (* (`self.VelocityRot`) DeltaSeconds)) false false)
  (`SceneComponent.K2_SetRelativeRotation` (`self.Empty`) (`KismetMathLibrary.MakeRotator` _returnvalue_2 _returnvalue_2 _returnvalue_4) false false)
  (`SceneComponent.K2_SetRelativeRotation` (`self.Empty_1`) (`KismetMathLibrary.MakeRotator` _returnvalue_3 _returnvalue_3 (* _returnvalue_4 -1.0)) false false))

(fn `UserConstructionScript`)