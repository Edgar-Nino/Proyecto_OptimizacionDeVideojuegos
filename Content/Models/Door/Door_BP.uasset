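; Door actor that the player can toggle open and closed once every Llave_BP key is gone from the level.
; On box overlap by BP_GRFH1_CharacterP, it sets the character's UI text to a Spanish hint and enables input only if no keys remain.
; A FlipFlop on Interaction plays or reverses a timeline that moves the door.
; Leaving clears the text, disables input and resets the overlap DoOnce.
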(event `InputAction|Interaction`
  (params (Key :type "Key Structure"))
  (:`Pressed`
    (`/Engine/EditorBlueprintResources/StandardMacros.FlipFlop`
      (:`A`
        (bind (_direction _value_close) (`Timeline|Cerrar Puerta` :!label _label)
          (:`Update`
            (`SceneComponent.K2_SetRelativeLocation` (`self.Door`) _value_close false false))))
      (:`B`
        (goto _label :!via `Reverse`)))))

(event `self.Box.OnComponentBeginOverlap`
  (params (OverlappedComponent :type "PrimitiveComponent Object Reference") (OtherActor :type "Actor Object Reference") (OtherComp :type "PrimitiveComponent Object Reference") (OtherBodyIndex :type Integer) (bFromSweep :type Boolean) (SweepResult :type "HitResult Structure (by ref)"))
  (`/Engine/EditorBlueprintResources/StandardMacros.DoOnce` false :!label _label_2
    (:`Completed`
      (if (== (`GameplayStatics.GetObjectClass` OtherActor) "/Game/GR_Stylized_Female_01/Character/Blueprints/BP_GRFH1_CharacterP.BP_GRFH1_CharacterP_C")
        (bind _outactors (`GameplayStatics.GetAllActorsOfClass` "/Game/Models/Llave/Llave_BP.Llave_BP_C"))
        (if (> (`KismetArrayLibrary.Array_Length` _outactors) 0)
          (bind _asbp_grfh1_character_p (cast `/Game/GR_Stylized_Female_01/Character/Blueprints/BP_GRFH1_CharacterP` OtherActor))
          (set `/Game/UI/UI.Text` "Recoge todas las llaves para abrir la puerta" (`/Game/GR_Stylized_Female_01/Character/Blueprints/BP_GRFH1_CharacterP.UI` _asbp_grfh1_character_p))
          (else
            (`self.EnableInput` (`GameplayStatics.GetPlayerController` 0))
            (bind _asbp_grfh1_character_p_2 (cast `/Game/GR_Stylized_Female_01/Character/Blueprints/BP_GRFH1_CharacterP` OtherActor))
            (set `/Game/UI/UI.Text` "Presiona e para abrir la puerta" (`/Game/GR_Stylized_Female_01/Character/Blueprints/BP_GRFH1_CharacterP.UI` _asbp_grfh1_character_p_2))))))))

(event `self.Box.OnComponentEndOverlap`
  (params (OverlappedComponent :type "PrimitiveComponent Object Reference") (OtherActor :type "Actor Object Reference") (OtherComp :type "PrimitiveComponent Object Reference") (OtherBodyIndex :type Integer))
  (if (== (`GameplayStatics.GetObjectClass` OtherActor) "/Game/GR_Stylized_Female_01/Character/Blueprints/BP_GRFH1_CharacterP.BP_GRFH1_CharacterP_C")
    (`self.DisableInput` (`GameplayStatics.GetPlayerController` 0))
    (bind _asbp_grfh1_character_p (cast `/Game/GR_Stylized_Female_01/Character/Blueprints/BP_GRFH1_CharacterP` (stale `self.Box.OnComponentBeginOverlap` OtherActor)))
    (set `/Game/UI/UI.Text` "" (`/Game/GR_Stylized_Female_01/Character/Blueprints/BP_GRFH1_CharacterP.UI` _asbp_grfh1_character_p))
    (goto _label_2 :!via `Reset`)))

(fn `UserConstructionScript`)