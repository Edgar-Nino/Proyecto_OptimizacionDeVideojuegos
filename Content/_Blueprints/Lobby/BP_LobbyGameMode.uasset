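; Lobby game mode for a Steam multiplayer session that tracks connected players and launches the match through server travel.
; PostLogin registers players and pulls session settings from the game instance, then interface messages push map settings, player info and available characters to each lobby controller.
; It also checks character selection for start readiness, spawns chosen characters at random PlayerStarts, handles kicks and updates character availability on logout.
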(event `self.K2_PostLogin`
  (params (NewPlayer :type "PlayerController Object Reference"))
  (bind _output_get (set `self.ConnectedPlayer` NewPlayer))
  (`KismetArrayLibrary.Array_AddUnique` (`self.ConnectedPlayers`) _output_get)
  (bind _outactors (`GameplayStatics.GetAllActorsOfClass` "/Script/Engine.PlayerStart"))
  (set `self.SpawnPoints` _outactors)
  (bind _gameinstance (message `/Game/_Blueprints/BPI_GameInstance.SteamGameInstanceRef` (`GameplayStatics.GetGameInstance`)))
  (set `self.ServerName` (`/Game/_Blueprints/SteamGameInstance.ServerName` _gameinstance))
  (set `self.MaxPlayers` (`/Game/_Blueprints/SteamGameInstance.NumberOfPlayers` _gameinstance))
  (bind _lobbypc (message `/Game/_Blueprints/Lobby/BPI_LobbyPC.Lobby_PCRef` (`self.ConnectedPlayer`)))
  (`/Game/_Blueprints/Lobby/BP_LobbyPC.InitialSetup` _lobbypc (`self.ServerName`) (`self.SelectedMapImage`) (`self.SelectedMapName`) (`self.SelectedMapTime`)))

(event `SpawnPlayer`
  (params (Player :type "PlayerController Object Reference")))

(event `StartLoadingScreen`
  (for _array_element (`self.ConnectedPlayers`)
    (bind _lobbypc (message `/Game/_Blueprints/Lobby/BPI_LobbyPC.Lobby_PCRef` _array_element))
    (`/Game/_Blueprints/Lobby/BP_LobbyPC.ShowLoadingScreen` _lobbypc)
    (`self.LaunchGame`)))

(event `EveryoneUpdate`
  (bind _connectedplayers (`self.ConnectedPlayers`))
  (bind _output_get (set `self.CurrentPlayers` (`KismetArrayLibrary.Array_Length` (`self.ConnectedPlayers`))))
  (if (> _output_get 0)
    (`KismetArrayLibrary.Array_Clear` (`self.ConnectedPlayersInfo`))
    (for _array_element _connectedplayers
      (bind _lobbypc (message `/Game/_Blueprints/Lobby/BPI_LobbyPC.Lobby_PCRef` _array_element))
      (`KismetArrayLibrary.Array_AddUnique` (`self.ConnectedPlayersInfo`) (`/Game/_Blueprints/Lobby/BP_LobbyPC.PlayerSettings` _lobbypc))
      (`/Game/_Blueprints/Lobby/BP_LobbyPC.UpdateNumberOfPlayers` _lobbypc (`self.CurrentPlayers`) (`self.MaxPlayers`)))
    (for _array_element_2 _connectedplayers
      (bind _lobbypc_2 (message `/Game/_Blueprints/Lobby/BPI_LobbyPC.Lobby_PCRef` _array_element_2))
      (`/Game/_Blueprints/Lobby/BP_LobbyPC.AddPlayerInfo` _lobbypc_2 (`self.ConnectedPlayersInfo`))
      (`/Game/_Blueprints/Lobby/BP_LobbyPC.UpdateAvailableCharacters` _lobbypc_2 (`self.AvailableCharacters`))
      (`/Game/_Blueprints/Lobby/BP_LobbyPC.UpdateColorCharacter` _lobbypc_2)
      (`self.AddToKickList`))
    (for _array_element_3 (`self.ConnectedPlayersInfo`) :!label _label
      (if (== (`.PlayerCharacter_16_6EA448244137B4356C465E9BAE8C4E0F` (break `/Game/_Blueprints/S_PlayerInfo` _array_element_3)) null)
        (set `self.CanWeStart?` false)
        (`self.CannotStartGame`)
        (else
          (set `self.CanWeStart?` true))))))

(event `CannotStartGame`
  (goto _label :!via `Break`))

(event `HostUpdateGameSettings`
  (params (SelectedMapTime :type Text) (SelectedMapImage :type "Texture2D Object Reference") (SelectedMapName :type Text) (SelectedMapID :type Integer))
  (set `self.SelectedMapImage` SelectedMapImage)
  (set `self.SelectedMapName` SelectedMapName)
  (set `self.SelectedMapID` SelectedMapID)
  (set `self.SelectedMapTime` SelectedMapTime)
  (for _array_element (`self.ConnectedPlayers`)
    (bind _lobbypc (message `/Game/_Blueprints/Lobby/BPI_LobbyPC.Lobby_PCRef` _array_element))
    (`/Game/_Blueprints/Lobby/BP_LobbyPC.UpdateLobbySettings` _lobbypc (`self.SelectedMapImage`) (`self.SelectedMapName`) (`self.SelectedMapTime`))))

(event `PlayerKicked`
  (params (PlayerID :type Integer))
  (bind _lobbypc (message `/Game/_Blueprints/Lobby/BPI_LobbyPC.Lobby_PCRef` (`|GetArrayItem` (`self.ConnectedPlayers`) PlayerID)))
  (`/Game/_Blueprints/Lobby/BP_LobbyPC.Kicked` _lobbypc))

(event `AddToKickList`
  (bind _lobbypc (message `/Game/_Blueprints/Lobby/BPI_LobbyPC.Lobby_PCRef` (`GameplayStatics.GetPlayerController` 0)))
  (`/Game/_Blueprints/Lobby/BP_LobbyPC.AddPlayerToKickWindow` _lobbypc))

(event `self.K2_OnLogout`
  (params (ExitingController :type "Controller Object Reference"))
  (bind _connectedplayers (`self.ConnectedPlayers`))
  (for (_array_element _array_index) _connectedplayers
    (if (== _array_element ExitingController)
      (break)))
  (bind _lobbypc (message `/Game/_Blueprints/Lobby/BPI_LobbyPC.Lobby_PCRef` (`|GetArrayItem` _connectedplayers _array_index)))
  (`KismetArrayLibrary.Array_Set` (`self.AvailableCharacters`) (`/Game/_Blueprints/Lobby/BP_LobbyPC.SelectedCharacter` _lobbypc))
  (`KismetArrayLibrary.Array_Remove` (`self.ConnectedPlayers`) _array_index)
  (`KismetArrayLibrary.Array_Remove` (`self.ConnectedPlayersInfo`) _array_index)
  (`self.EveryoneUpdate`))

(event `LaunchGame`
  (bind _returnvalue (`GameplayStatics.GetPlayerController` 0))
  (switch `int` (`self.SelectedMapID`)
    (:`0`
      (`KismetSystemLibrary.ExecuteConsoleCommand` "servertravel/Game/Level/NIVELn30n" _returnvalue))
    (:`1`
      (`KismetSystemLibrary.ExecuteConsoleCommand` "servertravel/Game/Level/NIVELn30n" _returnvalue))))

(event `ChangeCharacter`
  (params (ConnectedPlayer :type "PlayerController Object Reference") (CharacterClass :type "Character Class Reference") (`ChangedStatus?` :type Boolean) (Color :type String))
  (bind _returnvalue (`Controller.K2_GetPawn` ConnectedPlayer))
  (bind _spawnpoints (`self.SpawnPoints`))
  (if (not `ChangedStatus?`)
    (`/Engine/EditorBlueprintResources/StandardMacros.IsValid` _returnvalue
      (:`Is Valid`
        (`self.K2_DestroyActor` _returnvalue))
      (:`Is Not Valid`
        _))
    (bind _returnvalue_2 (`|SpawnActorFromClass` CharacterClass (`self.GetTransform` (`|GetArrayItem` _spawnpoints (`KismetMathLibrary.RandomInteger` (- (`KismetArrayLibrary.Array_Length` _spawnpoints) 1)))) "AlwaysSpawn" "OverrideRootScale" null null))
    (`Controller.Possess` ConnectedPlayer _returnvalue_2)))

(event `PauseAllPlayers`)

(fn `LobbyGMref`
  (returns (LobbyGM :type "/Game/_Blueprints/Lobby/BP_LobbyGameMode Object Reference"))
  (return self))

(fn `UserConstructionScript`)