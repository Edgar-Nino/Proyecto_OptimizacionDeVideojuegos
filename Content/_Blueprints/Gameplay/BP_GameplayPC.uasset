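; Multiplayer gameplay player controller that carries each player's saved profile, score, life and alive state through a match.
; On local BeginPlay it loads the save, passes it toward the game mode for pawn spawning, then builds chat and HUD widgets after a delay.
; Stat changes and chat route through the game mode interface for broadcast.
; It also handles winner display, session exit and shared pause that only the pausing player can release.
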(event `UpdateGame`)

(event `self.ReceiveBeginPlay`
  (if (`self.IsLocalController`)
    (`WidgetLayoutLibrary.RemoveAllWidgets`)
    (`self.LoadGame`)))

(event `LoadGame`
  (`KismetSystemLibrary.PrintString` "Hello")
  (bind _returnvalue (`GameplayStatics.LoadGameFromSlot` (`self.PlayerSettingsSave`)))
  (bind _asplayer_save (cast `/Game/_Blueprints/PlayerSave` _returnvalue))
  (bind (_playername _playerimage _playercharacter _characterimage _playerstatus _color) (break `/Game/_Blueprints/S_PlayerInfoW` (`/Game/_Blueprints/PlayerSave.PlayerInfo` _asplayer_save)))
  (bind _output_get (set `self.PlayerSettings` (make `/Game/_Blueprints/S_PlayerInfoW` _playername _playerimage _playercharacter _characterimage _playerstatus _color 0 true)))
  (`self.PassCharacterInfoToServer` _output_get))

(event `PassCharacterInfoToServer`
  (params (PlayerSettings :type "/Game/_Blueprints/S_PlayerInfoW Structure"))
  (bind _output_get (set `self.PlayerSettings` PlayerSettings))
  (bind _gameplaygmref (message `/Game/_Blueprints/Gameplay/BPI_GameplayGM.GameplayGMRef` (`GameplayStatics.GetGameMode`)))
  (bind (_playername _playerimage _playercharacter _characterimage _playerstatus _color) (break `/Game/_Blueprints/S_PlayerInfoW` _output_get))
  (`/Game/_Blueprints/Gameplay/BP_GameplayGameMode.SpawnPlayer` _gameplaygmref self _playercharacter _color)
  (`KismetSystemLibrary.Delay` 1.0)
  (`self.SetupUI`)
  (`/Game/_Blueprints/Gameplay/BP_GameplayGameMode.EveryoneUpdateColorSuit` _gameplaygmref))

(event `UpdateScore`
  (params (Score :type Integer))
  (bind _playersettings (`self.PlayerSettings`))
  (setmembers `/Game/_Blueprints/S_PlayerInfoW` :`StructRef` _playersettings :`Score` (+ (`.Score_23_CF5EA2894CF57EC25EAFB6B43DFF00E3` (break `/Game/_Blueprints/S_PlayerInfoW` _playersettings)) Score))
  (bind _gameplaygmref (message `/Game/_Blueprints/Gameplay/BPI_GameplayGM.GameplayGMRef` (`GameplayStatics.GetGameMode`)))
  (`/Game/_Blueprints/Gameplay/BP_GameplayGameMode.EveryoneUpdate` _gameplaygmref))

(event `UpdateLife`
  (params (Life :type "Float (double-precision)"))
  (bind _playersettings (`self.PlayerSettings`))
  (bind _returnvalue (- (`.Life_28_1505EED74108B0F3AC95049881658F4F` (break `/Game/_Blueprints/S_PlayerInfoW` _playersettings)) Life))
  (setmembers `/Game/_Blueprints/S_PlayerInfoW` :`StructRef` _playersettings :`Life` _returnvalue)
  (bind _gameplaygmref (message `/Game/_Blueprints/Gameplay/BPI_GameplayGM.GameplayGMRef` (`GameplayStatics.GetGameMode`)))
  (`/Game/_Blueprints/Gameplay/BP_GameplayGameMode.EveryoneUpdate` _gameplaygmref)
  (if (<= _returnvalue 0.0)
    (`self.UpdateAliveCharacters`)))

(event `SetupUI`
  (bind _returnvalue (`|CreateWidget` "/Game/_Widgets/ChatGameplay.ChatGameplay_C"))
  (bind _output_get (set `self.GameplayChat` _returnvalue))
  (bind _returnvalue_2 (`|CreateWidget` "/Game/UI/UI.UI_C"))
  (`UserWidget.AddToViewport` _output_get 0)
  (`UserWidget.AddToViewport` _returnvalue_2 0)
  (bind _asbp_grfh1_character_p (cast `/Game/GR_Stylized_Female_01/Character/Blueprints/BP_GRFH1_CharacterP` (`self.K2_GetPawn`)))
  (bind _output_get_2 (set `/Game/GR_Stylized_Female_01/Character/Blueprints/BP_GRFH1_CharacterP.UI` _returnvalue_2 _asbp_grfh1_character_p))
  (set `self.UIWidget` _output_get_2))

(event `UpdateAliveCharacters`
  (setmembers `/Game/_Blueprints/S_PlayerInfoW` :`StructRef` (`self.PlayerSettings`) :`Alive` false)
  (bind _gameplaygmref (message `/Game/_Blueprints/Gameplay/BPI_GameplayGM.GameplayGMRef` (`GameplayStatics.GetGameMode`)))
  (`/Game/_Blueprints/Gameplay/BP_GameplayGameMode.EveryoneUpdateAlive` _gameplaygmref))

(event `GetChatMessage`
  (params (TexToSend :type Text))
  (set `self.SenderText` TexToSend)
  (set `self.SenderName` (`.PlayerName_11_C473324C4A506DEA49AA9EAC1FAC5E34` (break `/Game/_Blueprints/S_PlayerInfoW` (`self.PlayerSettings`))))
  (bind _gameplaygmref (message `/Game/_Blueprints/Gameplay/BPI_GameplayGM.GameplayGMRef` (`GameplayStatics.GetGameMode`)))
  (`/Game/_Blueprints/Gameplay/BP_GameplayGameMode.UpdateChat` _gameplaygmref (`self.SenderText`) (`self.SenderName`)))

(event `UpdateChatWindow`
  (params (Sender :type Text) (Message :type Text)))

(event `Key|Enter`
  (params (Key :type "Key Structure"))
  (:`Pressed`
    (`/Engine/EditorBlueprintResources/StandardMacros.FlipFlop`
      (:`A`
        (set `self.bShowMouseCursor` true))
      (:`B`
        (set `self.bShowMouseCursor` false)))))

(event `UpdateColorCharacter`
  (bind _asbp_grfh1_character_p (cast `/Game/GR_Stylized_Female_01/Character/Blueprints/BP_GRFH1_CharacterP` (`self.K2_GetPawn`)))
  (`/Game/GR_Stylized_Female_01/Character/Blueprints/BP_GRFH1_CharacterP.SetColorSuit` _asbp_grfh1_character_p (`.Color_20_FE4BB7BE49ADC21E8E853A821A099FC0` (break `/Game/_Blueprints/S_PlayerInfoW` (`self.PlayerSettings`)))))

(event `UpdateWInner`
  (params (Winner :type "/Game/_Blueprints/S_PlayerInfoW Structure") (PCWinner :type "/Game/_Blueprints/Gameplay/BP_GameplayPC Object Reference"))
  (bind ((`PlayerName_11_C473324C4A506DEA49AA9EAC1FAC5E34` _playername) (`Score_23_CF5EA2894CF57EC25EAFB6B43DFF00E3` _score)) (break `/Game/_Blueprints/S_PlayerInfoW` Winner))
  (bind _uiwidget (`self.UIWidget`))
  (`KismetSystemLibrary.PrintString` "Winner")
  (set `/Game/UI/UI.WinnerMessage` (`|FormatText` "The winner is: {User} with {Score} points" _playername _score) _uiwidget)
  (`WidgetSwitcher.SetActiveWidgetIndex` (`/Game/UI/UI.SwitchWidgets` _uiwidget) 3)
  (`WidgetBlueprintLibrary.SetInputMode_GameAndUIEx` self _uiwidget "DoNotLock" false)
  (set `self.bShowMouseCursor` true)
  (if (== PCWinner self)
    (set `/Game/UI/UI.WinnerText` "Winner" _uiwidget)
    (else
      (set `/Game/UI/UI.WinnerText` "Loser" _uiwidget))))

(event `UpdateScorePlayer`
  (bind ((`Score_23_CF5EA2894CF57EC25EAFB6B43DFF00E3` _score) (`Life_28_1505EED74108B0F3AC95049881658F4F` _life)) (break `/Game/_Blueprints/S_PlayerInfoW` (`self.PlayerSettings`)))
  (bind _asbp_grfh1_character_p (cast `/Game/GR_Stylized_Female_01/Character/Blueprints/BP_GRFH1_CharacterP` (`self.K2_GetPawn`)))
  (set `/Game/GR_Stylized_Female_01/Character/Blueprints/BP_GRFH1_CharacterP.ScoreDisplay` _score _asbp_grfh1_character_p)
  (set `/Game/GR_Stylized_Female_01/Character/Blueprints/BP_GRFH1_CharacterP.Vida` _life _asbp_grfh1_character_p))

(event `UpdateAlive`
  (bind _asbp_grfh1_character_p (cast `/Game/GR_Stylized_Female_01/Character/Blueprints/BP_GRFH1_CharacterP` (`self.K2_GetPawn`)))
  (set `/Game/GR_Stylized_Female_01/Character/Blueprints/BP_GRFH1_CharacterP.Alive` (`.Alive_25_C0E288DD4A16EDFAB394699856121C8A` (break `/Game/_Blueprints/S_PlayerInfoW` (`self.PlayerSettings`))) _asbp_grfh1_character_p))

(event `ContinueBtn`
  (`self.PauseToServer` (`.PlayerName_11_C473324C4A506DEA49AA9EAC1FAC5E34` (break `/Game/_Blueprints/S_PlayerInfoW` (`self.PlayerSettings`))) self :!label _label))

(event `Key|P` :paused true :overrideparent false
  (params (Key :type "Key Structure"))
  (:`Pressed`
    (goto _label)))

(event `PauseToServer`
  (params (UserPause :type Text) (Controller :type "/Game/_Blueprints/Gameplay/BP_GameplayPC Object Reference"))
  (bind _gameplaygmref (message `/Game/_Blueprints/Gameplay/BPI_GameplayGM.GameplayGMRef` (`GameplayStatics.GetGameMode`)))
  (bind _ispaused_ (`/Game/_Blueprints/Gameplay/BP_GameplayGameMode.IsPaused?` _gameplaygmref))
  (if _ispaused_
    (if (== Controller (`/Game/_Blueprints/Gameplay/BP_GameplayGameMode.PCPause` _gameplaygmref))
      (bind _output_get (set `/Game/_Blueprints/Gameplay/BP_GameplayGameMode.IsPaused?` (not _ispaused_) _gameplaygmref :!label _label_2))
      (bind _allplayercontrollers (`/Game/_Blueprints/Gameplay/BP_GameplayGameMode.AllPlayerControllers` _gameplaygmref))
      (bind _returnvalue (`KismetArrayLibrary.Array_LastIndex` _allplayercontrollers))
      (for _index (range (+ _returnvalue 1))
        (bind _gameplaypc (message `/Game/_Blueprints/Gameplay/BPI_GameplayPC.GameplayPCref` (`|GetArrayItem` _allplayercontrollers (- _returnvalue _index))))
        (`self.PauseEvent` _gameplaypc _output_get UserPause)))
    (else
      (set `/Game/_Blueprints/Gameplay/BP_GameplayGameMode.PCPause` Controller _gameplaygmref)
      (goto _label_2))))

(event `PauseEvent`
  (params (Pause :type Boolean) (UserPause :type Text))
  (`/Game/UI/UI.Pause` (`self.UIWidget`) Pause UserPause)
  (`GameplayStatics.SetGamePaused` Pause)
  (if Pause
    (`WidgetBlueprintLibrary.SetInputMode_UIOnlyEx` self null)
    (set `self.bShowMouseCursor` true)
    (else
      (`WidgetBlueprintLibrary.SetInputMode_GameAndUIEx` self null)
      (set `self.bShowMouseCursor` false))))

(event `ExitBtn`
  (`DestroySessionCallbackProxy.DestroySession` self
    (:`OnSuccess`
      (`GameplayStatics.OpenLevel` "MainMenu"))))

(fn `GameplayPCref`
  (returns (GameplayPC :type "/Game/_Blueprints/Gameplay/BP_GameplayPC Object Reference"))
  (return self))

(fn `UserConstructionScript`)