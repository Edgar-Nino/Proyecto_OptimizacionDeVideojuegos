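; Multiplayer gameplay GameMode that tracks player controllers, spawns players at random PlayerStarts and relays match state to everyone.
; Update events rebuild the player info list from each controller's settings, then push suit color, score, alive status or chat through interface references.
; The alive update counts survivors and broadcasts the winner when only one remains.
; Logout asks the Steam game instance to destroy the exiting controller's session.
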(event `EveryoneUpdateWInner`
  (bind _allplayercontrollers (`self.AllPlayerControllers`))
  (`KismetArrayLibrary.Array_Clear` (`self.AllPlayerInfo`))
  (for _array_element _allplayercontrollers
    (bind _gameplaypc (message `/Game/_Blueprints/Gameplay/BPI_GameplayPC.GameplayPCref` _array_element))
    (`KismetArrayLibrary.Array_AddUnique` (`self.AllPlayerInfo`) (`/Game/_Blueprints/Gameplay/BP_GameplayPC.PlayerSettings` _gameplaypc)))
  (for _array_element_2 _allplayercontrollers
    (bind _gameplaypc_2 (message `/Game/_Blueprints/Gameplay/BPI_GameplayPC.GameplayPCref` _array_element_2))
    (`/Game/_Blueprints/Gameplay/BP_GameplayPC.UpdateWInner` _gameplaypc_2 (`self.LastPlayerAlive`) (`self.WinnerController`))))

(event `EveryoneUpdateColorSuit`
  (bind _allplayercontrollers (`self.AllPlayerControllers`))
  (`KismetArrayLibrary.Array_Clear` (`self.AllPlayerInfo`))
  (for _array_element _allplayercontrollers
    (bind _gameplaypc (message `/Game/_Blueprints/Gameplay/BPI_GameplayPC.GameplayPCref` _array_element))
    (`KismetArrayLibrary.Array_AddUnique` (`self.AllPlayerInfo`) (`/Game/_Blueprints/Gameplay/BP_GameplayPC.PlayerSettings` _gameplaypc)))
  (for _array_element_2 _allplayercontrollers
    (bind _gameplaypc_2 (message `/Game/_Blueprints/Gameplay/BPI_GameplayPC.GameplayPCref` _array_element_2))
    (`/Game/_Blueprints/Gameplay/BP_GameplayPC.UpdateColorCharacter` _gameplaypc_2)))

(event `EveryoneUpdateAlive`
  (bind _allplayercontrollers (`self.AllPlayerControllers`))
  (`KismetArrayLibrary.Array_Clear` (`self.AllPlayerInfo`))
  (set `self.Acumulado` 0)
  (for _array_element _allplayercontrollers
    (bind _gameplaypc (message `/Game/_Blueprints/Gameplay/BPI_GameplayPC.GameplayPCref` _array_element))
    (bind _playersettings (`/Game/_Blueprints/Gameplay/BP_GameplayPC.PlayerSettings` _gameplaypc))
    (`KismetArrayLibrary.Array_AddUnique` (`self.AllPlayerInfo`) _playersettings)
    (if (`.Alive_25_C0E288DD4A16EDFAB394699856121C8A` (break `/Game/_Blueprints/S_PlayerInfoW` _playersettings))
      (set `self.Acumulado` (+ (`self.Acumulado`) 1))
      (set `self.LastPlayerAlive` _playersettings)
      (set `self.WinnerController` _gameplaypc)))
  (for _array_element_2 _allplayercontrollers
    (bind _gameplaypc_2 (message `/Game/_Blueprints/Gameplay/BPI_GameplayPC.GameplayPCref` _array_element_2))
    (`/Game/_Blueprints/Gameplay/BP_GameplayPC.UpdateAlive` _gameplaypc_2)
    (if (== (`self.Acumulado`) 1)
      (`self.EveryoneUpdateWInner`))))

(event `EveryoneUpdate`
  (bind _allplayercontrollers (`self.AllPlayerControllers`))
  (`KismetArrayLibrary.Array_Clear` (`self.AllPlayerInfo`))
  (for _array_element _allplayercontrollers
    (bind _gameplaypc (message `/Game/_Blueprints/Gameplay/BPI_GameplayPC.GameplayPCref` _array_element))
    (`KismetArrayLibrary.Array_AddUnique` (`self.AllPlayerInfo`) (`/Game/_Blueprints/Gameplay/BP_GameplayPC.PlayerSettings` _gameplaypc)))
  (for _array_element_2 _allplayercontrollers
    (bind _gameplaypc_2 (message `/Game/_Blueprints/Gameplay/BPI_GameplayPC.GameplayPCref` _array_element_2))
    (`/Game/_Blueprints/Gameplay/BP_GameplayPC.UpdateScorePlayer` _gameplaypc_2)))

(event `SpawnPlayer`
  (params (PlayerController :type "PlayerController Object Reference") (CharacterClass :type "Character Class Reference") (Color :type String))
  (bind _returnvalue (`Controller.K2_GetPawn` PlayerController))
  (bind _spawnpoints (`self.SpawnPoints`))
  (bind _outactors (`GameplayStatics.GetAllActorsOfClass` "/Script/Engine.PlayerStart"))
  (set `self.SpawnPoints` _outactors)
  (`/Engine/EditorBlueprintResources/StandardMacros.IsValid` _returnvalue
    (:`Is Valid`
      (`self.K2_DestroyActor` _returnvalue))
    (:`Is Not Valid`
      _))
  (bind _returnvalue_2 (`|SpawnActorFromClass` CharacterClass (`self.GetTransform` (`|GetArrayItem` _spawnpoints (`KismetMathLibrary.RandomInteger` (- (`KismetArrayLibrary.Array_Length` _spawnpoints) 1)))) "AlwaysSpawn" "OverrideRootScale" null null))
  (`Controller.Possess` PlayerController _returnvalue_2))

(event `self.K2_OnSwapPlayerControllers`
  (params (OldPC :type "PlayerController Object Reference") (NewPC :type "PlayerController Object Reference"))
  (`KismetArrayLibrary.Array_Add` (`self.AllPlayerControllers`) NewPC)
  (`self.EveryoneUpdateColorSuit`))

(event `self.K2_OnLogout`
  (params (ExitingController :type "Controller Object Reference"))
  (bind _gameplaypc (message `/Game/_Blueprints/Gameplay/BPI_GameplayPC.GameplayPCref` ExitingController))
  (bind _gameinstance (message `/Game/_Blueprints/BPI_GameInstance.SteamGameInstanceRef` (`GameplayStatics.GetGameInstance`)))
  (message `/Game/_Blueprints/BPI_GameInstance.DestroySessionCaller` _gameinstance _gameplaypc))

(event `UpdateChat`
  (params (Sender :type Text) (Message :type Text))
  (for _array_element (`self.AllPlayerControllers`)
    (bind _gameplaypc (message `/Game/_Blueprints/Gameplay/BPI_GameplayPC.GameplayPCref` _array_element))
    (`/Game/_Blueprints/Gameplay/BP_GameplayPC.UpdateChatWindow` _gameplaypc Sender Message)))

(fn `GameplayGMRef`
  (returns (GameplayGMRef :type "/Game/_Blueprints/Gameplay/BP_GameplayGameMode Object Reference"))
  (return self))

(fn `UserConstructionScript`)